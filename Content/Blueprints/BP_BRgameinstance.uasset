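; Game instance Blueprint that handles session matchmaking, joining an existing game or hosting a new one.
; The try-join-or-create event searches for sessions using the UseLan setting, joins the first result, and creates a session if none exist or the search fails.
; Hosting opens the Overview level as a listen server.
; Successful hosting or joining hides the cursor and sets game-only input, while failures print an error.
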(event `try join or creat game`
  (bind _returnvalue (`GameplayStatics.GetPlayerController` 0))
  ;[1 1 1] try join creat session
  (bind _results (`FindSessionsCallbackProxy.FindSessions` (`GameplayStatics.GetPlayerController` 0) 20 (`self.Use Lan?`))
    (:`then`
      (if (`KismetArrayLibrary.Array_IsValidIndex` _results)
        (`self.join BP session` (`|GetArrayItem` _results))
        (else
          (`CreateSessionCallbackProxy.CreateSession` (`GameplayStatics.GetPlayerController` 0) 20 (`self.Use Lan?`) :!label _label
            (:`OnSuccess`
              (`GameplayStatics.OpenLevel` "Overview" true "Listen")
              (set `PlayerController.bShowMouseCursor` false _returnvalue)
              (`WidgetBlueprintLibrary.SetInputMode_GameOnly` _returnvalue))
            (:`OnFailure`
              (`KismetSystemLibrary.PrintString` "ERROR CREATING SESSION"))))))
    (:`OnFailure`
      (goto _label))))

(event `join BP session`
  (params (session :type "BlueprintSessionResult Structure"))
  (bind _returnvalue (`GameplayStatics.GetPlayerController` 0))
  ;[1 1 1] join session
  (`JoinSessionCallbackProxy.JoinSession` (`GameplayStatics.GetPlayerController` 0) session
    (:`OnSuccess`
      (set `PlayerController.bShowMouseCursor` false _returnvalue)
      (`WidgetBlueprintLibrary.SetInputMode_GameOnly` _returnvalue))
    (:`OnFailure`
      (`KismetSystemLibrary.PrintString` "ERROR JOINING SESSION"))))