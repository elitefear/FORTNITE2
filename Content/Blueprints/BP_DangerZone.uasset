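; Battle royale safe zone that registers with BR_gamestate and damages players left outside its shrinking wall.
; Once enabled, the server alternates timed holds and shrinks, picking a random offset center and scaling radius and durations each round until below the minimum radius.
; Tick scales and moves the wall toward that center.
; Capsule overlaps set each character's Inzone flag, which the server checks across living players to apply per-frame damage.
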(event `self.ReceiveBeginPlay`
  (`/Engine/EditorBlueprintResources/ActorMacros.Switch Has Authority`
    (:`Authority`
      (bind _asbr_gamestate (cast `/Game/FirstPersonBP/Blueprints/BR_gamestate` (`GameplayStatics.GetGameState`)))
      (set `/Game/FirstPersonBP/Blueprints/BR_gamestate.SafeZone` self _asbr_gamestate)
      (set `self.NextRadius` (* (`self.radius`) (`self.shrinkmultiplyer`)))
      (set `self.shrinkspeed` (/ (- (`self.radius`) (`self.NextRadius`)) (`self.shrinktime`)))
      (set `self.nextlocation` (`self.Getnextlocation`)))))

(event `begin shrinking`
  (`/Engine/EditorBlueprintResources/ActorMacros.Switch Has Authority`
    (:`Authority`
      (`/Engine/EditorBlueprintResources/StandardMacros.IncrementInt` (`self.NumShrinks`)
        (:`  `
          (set `self.Startshrinklocation` (`self.K2_GetActorLocation`))
          (set `self.shrinking?` true)
          (set `self.beginshrinktime` (`GameplayStatics.GetTimeSeconds`))
          (set `self.shrinkspeed` (/ (- (`self.radius`) (`self.NextRadius`)) (`self.shrinktime`)))
          (`self.SetActorHiddenInGame` false))))))

(event `enable safe zone`
  (`/Engine/EditorBlueprintResources/ActorMacros.Switch Has Authority`
    (:`Authority`
      (set `self.enabled?` true)
      (`KismetSystemLibrary.K2_SetTimerDelegate` (delegate `begin shrinking`) (`self.holdtime`)))))

(event `self.ReceiveTick`
  (params (DeltaSeconds :type "Float (single-precision)"))
  (if (`self.shrinking?`)
    (`self.Update wall transform` DeltaSeconds))
  (if (`self.enabled?`)
    (`/Engine/EditorBlueprintResources/ActorMacros.Switch Has Authority`
      (:`Authority`
        (`self.damage player outside wall` DeltaSeconds)))))

(event `Update wall transform`
  (params (deltaseconds :type "Float (double-precision)"))
  (bind _radius (`self.radius`))
  (set `self.radius` (- (`self.radius`) (* (`self.shrinkspeed`) deltaseconds)))
  (`self.SetActorScale3D` (`KismetMathLibrary.MakeVector` _radius _radius (`self.hight`)))
  (`self.K2_SetActorLocation` (`KismetMathLibrary.VInterpTo_Constant` (`self.K2_GetActorLocation`) (`self.nextlocation`) (stale `self.ReceiveTick` DeltaSeconds) (/ (`KismetMathLibrary.VSize` (- (`self.Startshrinklocation`) (`self.nextlocation`))) (`self.shrinktime`))))
  (if (and (`self.HasAuthority`) (>= (/ (- (`GameplayStatics.GetTimeSeconds`) (`self.beginshrinktime`)) (`self.shrinktime`)) 1.0))
    (set `self.shrinking?` false)
    (set `self.holdtime` (* (`self.holdtime`) (`self.timemultiplyer`)))
    (set `self.NextRadius` (* (`self.NextRadius`) (`self.shrinkmultiplyer`)))
    (set `self.nextlocation` (`self.Getnextlocation`))
    (set `self.shrinktime` (* (`self.shrinktime`) (`self.timemultiplyer`)))
    (if (>= (`self.radius`) (`self.minradius`))
      (`KismetSystemLibrary.K2_SetTimerDelegate` (delegate `begin shrinking`) (`self.holdtime`))
      (else
        (set `self.finishedshrinking?` true)))))

(event `self.Capsule.OnComponentBeginOverlap`
  (params (OverlappedComponent :type "PrimitiveComponent Object Reference") (OtherActor :type "Actor Object Reference") (OtherComp :type "PrimitiveComponent Object Reference") (OtherBodyIndex :type Integer) (bFromSweep :type Boolean) (SweepResult :type "HitResult Structure (by ref)"))
  (bind _asfirst_person_character (cast `/Game/FirstPersonBP/Blueprints/FirstPersonCharacter` OtherActor))
  (set `/Game/FirstPersonBP/Blueprints/FirstPersonCharacter.inzone?` true _asfirst_person_character))

(event `self.Capsule.OnComponentEndOverlap`
  (params (OverlappedComponent :type "PrimitiveComponent Object Reference") (OtherActor :type "Actor Object Reference") (OtherComp :type "PrimitiveComponent Object Reference") (OtherBodyIndex :type Integer))
  (bind _asfirst_person_character (cast `/Game/FirstPersonBP/Blueprints/FirstPersonCharacter` OtherActor))
  (set `/Game/FirstPersonBP/Blueprints/FirstPersonCharacter.inzone?` false _asfirst_person_character))

(event `damage player outside wall`
  (params (deltaseconds :type "Float (double-precision)"))
  (bind _returnvalue (* deltaseconds (+ (`self.timemultiplyer`) 1.0)))
  (bind _asgamemode_br (cast `/Game/FirstPersonBP/Blueprints/Gamemode_BR` (`GameplayStatics.GetGameMode`)))
  (for _array_element (`/Game/FirstPersonBP/Blueprints/Gamemode_BR.aliveplayerlist` _asgamemode_br)
    (bind _asfirst_person_character (cast `/Game/FirstPersonBP/Blueprints/FirstPersonCharacter` (`Controller.K2_GetPawn` _array_element)))
    (if (not (`/Game/FirstPersonBP/Blueprints/FirstPersonCharacter.inzone?` _asfirst_person_character))
      (`GameplayStatics.ApplyDamage` _asfirst_person_character _returnvalue)
      (`KismetSystemLibrary.PrintString` (`KismetStringLibrary.Conv_DoubleToString` _returnvalue)))))

(fn `Getnextlocation`
  (returns (nextlocation :type "Vector Structure"))
  (bind _returnvalue (`self.K2_GetActorLocation`))
  (bind _z (.z _returnvalue))
  (bind _returnvalue_2 (* (- (`self.radius`) (`self.NextRadius`)) 0.5))
  (bind _returnvalue_3 (* _returnvalue_2 -1.0))
  (return (`KismetMathLibrary.MakeVector` (.x (+ _returnvalue (`KismetMathLibrary.MakeVector` (* (`KismetMathLibrary.DegCos` (`KismetMathLibrary.RandomFloatInRange` -180.0 180.0)) (`KismetMathLibrary.RandomFloatInRange` _returnvalue_3 _returnvalue_2)) (* (`KismetMathLibrary.DegSin` (`KismetMathLibrary.RandomFloatInRange` -180.0 180.0)) (`KismetMathLibrary.RandomFloatInRange` _returnvalue_3 _returnvalue_2)) _z))) (.y (+ _returnvalue (`KismetMathLibrary.MakeVector` (* (`KismetMathLibrary.DegCos` (`KismetMathLibrary.RandomFloatInRange` -180.0 180.0)) (`KismetMathLibrary.RandomFloatInRange` _returnvalue_3 _returnvalue_2)) (* (`KismetMathLibrary.DegSin` (`KismetMathLibrary.RandomFloatInRange` -180.0 180.0)) (`KismetMathLibrary.RandomFloatInRange` _returnvalue_3 _returnvalue_2)) _z))) _z)))

(fn `UserConstructionScript`
  (bind _radius (`self.radius`))
  (`SceneComponent.SetWorldScale3D` (`self.Dangerzone`) (`KismetMathLibrary.MakeVector` _radius _radius (`self.hight`))))