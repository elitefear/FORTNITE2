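; BP_Weapon is a weapon Blueprint that tracks clip and spare ammo for its owning FirstPersonCharacter.
; On the server, it caches the owner at BeginPlay, spends a round per shot, reloads when empty and accepts added spare ammo.
; Reload flags the owner as reloading during a fixed delay, then fills the clip from spare ammo.
; HasAmmo reports whether rounds remain in the clip.
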(event `reload`
  (bind _returnvalue (`KismetMathLibrary.Min` (`self.current spare ammo`) (`self.clip size`)))
  ;[1 1 1] reload weapon and play animation
  (set `/Game/FirstPersonBP/Blueprints/FirstPersonCharacter.reloading?` true (`self.current owner`))
  (`KismetSystemLibrary.Delay` 2.0)
  (set `self.current ammo` _returnvalue)
  (set `self.current spare ammo` (`KismetMathLibrary.Max` (- (`self.current spare ammo`) _returnvalue)))
  (set `/Game/FirstPersonBP/Blueprints/FirstPersonCharacter.reloading?` false (`self.current owner`)))

(event `on fired`
  (bind _current_ammo (`self.current ammo`))
  ;[1 1 1] when fire gun take ammo from player and reload if neended
  (`/Engine/EditorBlueprintResources/ActorMacros.Switch Has Authority`
    (:`Authority`
      (`/Engine/EditorBlueprintResources/StandardMacros.DecrementInt` _current_ammo
        (:`  `
          (if (<= _current_ammo 0)
            (`self.reload`)))))))

(event `give ammo`
  (params (`ammo to give` :type Integer))
  ;[1 1 1] give ammo to weapon when needed
  (`/Engine/EditorBlueprintResources/ActorMacros.Switch Has Authority`
    (:`Authority`
      (set `self.current spare ammo` (+ `ammo to give` (`self.current spare ammo`))))))

(event `self.ReceiveBeginPlay`
  (`/Engine/EditorBlueprintResources/ActorMacros.Switch Has Authority`
    (:`Authority`
      (bind _asfirst_person_character (cast `/Game/FirstPersonBP/Blueprints/FirstPersonCharacter` (`self.GetOwner`)))
      (set `self.current owner` _asfirst_person_character))))

(fn `has ammo`
  (returns (`has ammo` :type Boolean))
  (return (> (`self.current ammo`) 0)))

(fn `UserConstructionScript`)