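; Base pickup Blueprint with a continuously spinning mesh and a sphere that detects the FirstPersonCharacter.
; Tick yaws the mesh at a constant rate and zeroes its world pitch and roll to keep it upright.
; The sphere disables its physics simulation on hit.
; Its overlaps pass the character to entered and left events, which are empty here.
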(event `self.ReceiveTick`
  (params (DeltaSeconds :type "Float (single-precision)"))
  (bind _pickupmesh (`self.pickupmesh`))
  ;[1 1 1] make pic up mesh spin
  (`SceneComponent.K2_AddRelativeRotation` _pickupmesh (`KismetMathLibrary.MakeRotator` 0.0 0.0 (* DeltaSeconds 180.0)) false false)
  (`SceneComponent.K2_SetWorldRotation` (`self.pickupmesh`) (`KismetMathLibrary.MakeRotator` 0.0 0.0 (.yaw (`SceneComponent.K2_GetComponentRotation` _pickupmesh))) false false))

(event `pick up sphere entered`
  (params (`charter ` :type "/Game/FirstPersonBP/Blueprints/FirstPersonCharacter Object Reference")))

(event `pickup sphere left`
  (params (charter :type "/Game/FirstPersonBP/Blueprints/FirstPersonCharacter Object Reference")))

(event `self.pickupmesh.OnComponentHit`
  (params (HitComponent :type "PrimitiveComponent Object Reference") (OtherActor :type "Actor Object Reference") (OtherComp :type "PrimitiveComponent Object Reference") (NormalImpulse :type "Vector Structure") (Hit :type "HitResult Structure (by ref)")))

(event `self.Sphere.OnComponentHit`
  (params (HitComponent :type "PrimitiveComponent Object Reference") (OtherActor :type "Actor Object Reference") (OtherComp :type "PrimitiveComponent Object Reference") (NormalImpulse :type "Vector Structure") (Hit :type "HitResult Structure (by ref)"))
  (`PrimitiveComponent.SetSimulatePhysics` (`self.Sphere`) false))

(event `self.Sphere.OnComponentBeginOverlap`
  (params (OverlappedComponent :type "PrimitiveComponent Object Reference") (OtherActor :type "Actor Object Reference") (OtherComp :type "PrimitiveComponent Object Reference") (OtherBodyIndex :type Integer) (bFromSweep :type Boolean) (SweepResult :type "HitResult Structure (by ref)"))
  (bind _asfirst_person_character (cast `/Game/FirstPersonBP/Blueprints/FirstPersonCharacter` OtherActor))
  (`self.pick up sphere entered` _asfirst_person_character))

(event `self.Sphere.OnComponentEndOverlap`
  (params (OverlappedComponent :type "PrimitiveComponent Object Reference") (OtherActor :type "Actor Object Reference") (OtherComp :type "PrimitiveComponent Object Reference") (OtherBodyIndex :type Integer))
  (bind _asfirst_person_character (cast `/Game/FirstPersonBP/Blueprints/FirstPersonCharacter` OtherActor))
  (`self.pickup sphere left` _asfirst_person_character))

(fn `UserConstructionScript`)