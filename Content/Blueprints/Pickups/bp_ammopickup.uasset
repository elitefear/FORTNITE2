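; Ammo pickup Blueprint that refills the spare ammo of a character's weapon when the character enters its pickup sphere.
; On the authority only, it checks for a valid weapon with room for more spare ammo, then calls GiveAmmo on it.
; If the full amount would exceed the maximum, it tops up the weapon and keeps the remainder; otherwise it gives everything and destroys itself.
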(event `self.pick up sphere entered`
  (params (`charter ` :type "/Game/FirstPersonBP/Blueprints/FirstPersonCharacter Object Reference"))
  (bind _weapon (`/Game/FirstPersonBP/Blueprints/FirstPersonCharacter.weapon` `charter `))
  (bind _maxspareammo (`/Game/Blueprints/weapons/BP_Weapon.maxspareammo` _weapon))
  (bind _current_spare_ammo (`/Game/Blueprints/weapons/BP_Weapon.current spare ammo` _weapon))
  (bind _returnvalue (- (`/Game/Blueprints/weapons/BP_Weapon.maxspareammo` _weapon) (`/Game/Blueprints/weapons/BP_Weapon.current spare ammo` _weapon)))
  (`/Engine/EditorBlueprintResources/ActorMacros.Switch Has Authority`
    (:`Authority`
      (`/Engine/EditorBlueprintResources/StandardMacros.IsValid` _weapon
        (:`Is Valid`
          (if (< _current_spare_ammo _maxspareammo)
            (if (> (+ (`self.ammotogive`) _current_spare_ammo) _maxspareammo)
              (set `self.ammotogive` (- (`self.ammotogive`) _returnvalue))
              (`/Game/Blueprints/weapons/BP_Weapon.give ammo` _weapon _returnvalue)
              (else
                (`/Game/Blueprints/weapons/BP_Weapon.give ammo` _weapon (`self.ammotogive`))
                (`self.K2_DestroyActor`)))))))))

(fn `UserConstructionScript`
  (`parent.UserConstructionScript`))