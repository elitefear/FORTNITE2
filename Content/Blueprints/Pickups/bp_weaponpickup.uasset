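; Weapon pickup Blueprint that represents a weapon a character can collect, along with the ammo it carries.
; On BeginPlay the server copies clip and spare ammo from the WeaponToGive class defaults, skipping this when the pickup was dropped by a player.
; Pickup sphere enter and leave events register the pickup as the character's current weapon pickup, clearing it on exit only if it is still the current one.
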(event `self.ReceiveBeginPlay`
  (bind (_damage _weaponname _current_ammo _current_spare_ammo) (defaults `/Game/Blueprints/Pickups/bp_weaponpickup` (`self.WeaponToGive`)))
  ;[1 1 1] remember ammo amounts
  (`/Engine/EditorBlueprintResources/ActorMacros.Switch Has Authority`
    (:`Authority`
      (if (not (`self.droppedbyplayer?`))
        (set `self.currentammoinclip` _current_ammo)
        (set `self.currentspareammo` _current_spare_ammo)))))

(event `self.pick up sphere entered`
  (params (`charter ` :type "/Game/FirstPersonBP/Blueprints/FirstPersonCharacter Object Reference"))
  ;[1 1 1] set playerpickup
  (set `/Game/FirstPersonBP/Blueprints/FirstPersonCharacter.currentweapnpickup` self `charter `))

(event `self.pickup sphere left`
  (params (charter :type "/Game/FirstPersonBP/Blueprints/FirstPersonCharacter Object Reference"))
  ;[1 1 1] unset player pick up
  (if (== (`/Game/FirstPersonBP/Blueprints/FirstPersonCharacter.currentweapnpickup` charter) self)
    (set `/Game/FirstPersonBP/Blueprints/FirstPersonCharacter.currentweapnpickup` null charter)))

(fn `UserConstructionScript`
  (`parent.UserConstructionScript`))