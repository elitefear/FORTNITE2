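; Health pickup Blueprint that heals a character entering its pickup sphere, then destroys itself.
; The PickUpSphereEntered event acts only with authority and only when the character is below max health.
; It passes the negated Healthtogive amount to the character's ModifyHealth and prints the resulting health.
; BeginPlay, overlap and Tick events are unused stubs.
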(event `self.pick up sphere entered`
  (params (`charter ` :type "/Game/FirstPersonBP/Blueprints/FirstPersonCharacter Object Reference"))
  (`/Engine/EditorBlueprintResources/ActorMacros.Switch Has Authority`
    (:`Authority`
      (if (< (`/Game/FirstPersonBP/Blueprints/FirstPersonCharacter.health` `charter `) (`/Game/FirstPersonBP/Blueprints/FirstPersonCharacter.Max health` `charter `))
        (`/Game/FirstPersonBP/Blueprints/FirstPersonCharacter.modify health` `charter ` (* (`self.healthtogive`) -1.0))
        (`KismetSystemLibrary.PrintString` (`KismetStringLibrary.Conv_DoubleToString` (`/Game/FirstPersonBP/Blueprints/FirstPersonCharacter.health` `charter `)))
        (`self.K2_DestroyActor`)))))

(fn `UserConstructionScript`
  (`parent.UserConstructionScript`))