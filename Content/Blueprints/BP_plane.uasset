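; Plane actor that flies across the map at a set height along a randomized straight path, with a spring arm set long and high.
; On BeginPlay the authority picks a random start MapSize/2 from the world origin and an opposite end skewed up to 15 degrees, then faces along it.
; Lifespan is MapSize over FlightSpeed.
; Tick, not authority-gated, moves it toward the end at constant speed, pinning Z to FlyHight.
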(event `self.ReceiveBeginPlay`
  (bind _springarm (`self.SpringArm`))
  ;[1 1 1] plane direction and hight
  (`/Engine/EditorBlueprintResources/ActorMacros.Switch Has Authority`
    (:`Authority`
      (set `SpringArmComponent.TargetArmLength` 3000.0 _springarm)
      (set `SpringArmComponent.TargetOffset` (0.0 0.0 1500.0) _springarm)
      (`self.SetLifeSpan` (/ (`self.map size`) (`self.flight speed`)))
      (bind _output_get (set `self.center offset` (`KismetMathLibrary.Normal` (`KismetMathLibrary.MakeVector` (`KismetMathLibrary.DegCos` (`KismetMathLibrary.RandomFloatInRange` -180.0 180.0)) (`KismetMathLibrary.DegSin` (`KismetMathLibrary.RandomFloatInRange` -180.0 180.0))))))
      (set `self.flight path start` (* _output_get (/ (`self.map size`) 2.0)))
      (set `self.flight path end` (* (`KismetMathLibrary.GreaterGreater_VectorRotator` (* (`self.center offset`) -1.0) (`KismetMathLibrary.MakeRotator` 0.0 0.0 (`KismetMathLibrary.RandomFloatInRange` -15.0 15.0))) (/ (`self.map size`) 2.0)))
      (`self.K2_SetActorRotation` (`KismetMathLibrary.Conv_VectorToRotator` (- (`self.flight path end`) (`self.flight path start`))))
      (`self.K2_SetActorLocation` (`self.flight path start`)))))

(event `self.ReceiveTick`
  (params (DeltaSeconds :type "Float (single-precision)"))
  ;[1 1 1] move plane
  (`self.K2_SetActorLocation` (`KismetMathLibrary.MakeVector` (.x (`KismetMathLibrary.VInterpTo_Constant` (`self.K2_GetActorLocation`) (`self.flight path end`) DeltaSeconds (`self.flight speed`))) (.y (`KismetMathLibrary.VInterpTo_Constant` (`self.K2_GetActorLocation`) (`self.flight path end`) DeltaSeconds (`self.flight speed`))) (`self.fly hight`))))

(fn `UserConstructionScript`)